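; BP_Dog is a VR dog actor that waits to be petted by the player's hand.
; While it is waiting, an overlap with any actor tagged "Hand" calls PetDog, which destroys the Advice actor and clears the waiting flag.
; PetDog then casts to GameInstanceVR and plays the dog (Perro) and UFO level sequences, reached through a collapsed graph fed by the VR player settings struct.
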(event Custom|PetDog
  (Actor|DestroyActor (Variables|Default|GetAdvice))
  (Variables|Default|SetisWaitingToBePet false)
  (bind _asgame_instance_vr (Utilities|Casting|CastToGameInstanceVR (Game|GetGameInstance)))
  (Sequencer|Player|Play (Variables|/Script/LevelSequence.LevelSequenceActor|GetSequencePlayer (.PerroSequence (|CollapseGraph_0 (Variables|/Game/VRContent/Core/GameInstanceVR.GameInstanceVR_C|GetStruc%20VR%20Player%20Settings _asgame_instance_vr)))) :!class /Script/MovieScene.MovieSceneSequencePlayer)
  (Sequencer|Player|Play (Variables|/Script/LevelSequence.LevelSequenceActor|GetSequencePlayer (.UfoSequence (|CollapseGraph_0 (Variables|/Game/VRContent/Core/GameInstanceVR.GameInstanceVR_C|GetStruc%20VR%20Player%20Settings _asgame_instance_vr)))) :!class /Script/MovieScene.MovieSceneSequencePlayer))

(event EventBeginPlay)

(event Collision|EventActorBeginOverlap
  (params (OtherActor :type Actor%20Object%20Reference))
  (if (Variables|Default|GetisWaitingToBePet)
    (if (Actor|ActorHasTag OtherActor "Hand")
      (CallFunction|PetDog))))

(fn ConstructionScript)